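; BP_HexGrid is a procedural hex-tile terrain generator that builds a Width by Height grid in its construction script, staggering alternate rows.
; Tiles are either mesh instances or BP_Tile child actors.
; Only instances get FastNoise-driven height, also written to custom data for the material; the second noise layer is configured but unused.
; A water plane is scaled from grid dimensions and positioned using the first and last instance transforms.
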(fn `UserConstructionScript`
  (locals (InstanceIndex :type Integer :default 0) (TimesRan :type Integer))
  (bind _noisescale (`self.NoiseScale`))
  (bind _first_transform_location (`KismetMathLibrary.BreakTransform` (`self.First Transform`)))
  (bind _final_transform_location (`KismetMathLibrary.BreakTransform` (`self.Final Transform`)))
  (bind _outinstancetransform (`InstancedStaticMeshComponent.GetInstanceTransform` (`self.InstancedStaticMesh`) (`local.InstanceIndex`) false))
  (bind (_returnvalue_x _returnvalue_y) (`KismetMathLibrary.BreakVector` (/ (- _final_transform_location _first_transform_location) 2.0)))
  (bind _returnvalue (`FastNoiseWrapper.GetNoise2D` (`self.NoiseWrapperLvl1`) (* (.x (.location _outinstancetransform)) _noisescale) (* (.y (.location _outinstancetransform)) _noisescale)))
  ;[1 1 1] Noise Level 1
  (bind _returnvalue_2 (`|GenericCreateObject` "/Script/FastNoiseGenerator.FastNoiseWrapper"))
  (bind _output_get (set `self.NoiseWrapperLvl1` _returnvalue_2))
  (`FastNoiseWrapper.SetupFastNoise` _output_get (`self.Noise Type`) (`self.Seed`) (`self.Frequency`) (`self.Interp`) (`self.Fractaltype`) (`self.Octaves`) (`self.Lacunarity`) (`self.Gain`) (`self.Cellular Jitter`) (`self.Cellular Distance Function`) (`self.Cellular Return Type`))
  ;[1 1 1] Noise Level 2
  (bind _returnvalue_3 (`|GenericCreateObject` "/Script/FastNoiseGenerator.FastNoiseWrapper"))
  (bind _output_get_2 (set `self.NoiseWrapperLvl2` _returnvalue_3))
  (`FastNoiseWrapper.SetupFastNoise` _output_get_2 (`self.Lvl 2 Noise Type`) (`self.Lvl 2 Seed`) (`self.Lvl 2 Frequency`) (`self.Lvl 2 Interp`) (`self.Lvl 2 Fractaltype`) (`self.Lvl 2 Octaves`) (`self.Lvl 2 Lacunarity`) (`self.Lvl 2 Gain`) (`self.Lvl 2 Cellular Jitter`) (`self.Lvl 2 Cellular Distance Function`) (`self.Lvl 2 Cellular Return Type`))
  (`StaticMeshComponent.SetStaticMesh` (`self.InstancedStaticMesh`) (`self.TitleMesh`))
  (set `self.Radius` (* (.x (`.Max` (break `Box` (`StaticMesh.GetBoundingBox` (`self.TitleMesh`))))) (`self.Scale`)))
  (for _index (range 1 (+ (`self.Height`) 1))
    (for _index_2 (range 1 (+ (`self.Width`) 1))
      (if (`self.IsInstanced`)
        (bind _returnvalue_4 (+ (* _index_2 (`self.Radius`) 2.0) (* _index_2 (`self.Offset`)) (`self.RowOffset`)))
        (bind _returnvalue_5 (+ (* _index (/ (* (`self.Radius`) 2.0) (`KismetMathLibrary.Sqrt` 3.0)) 1.5) (* _index (`self.Offset`))))
        (bind _returnvalue_6 (`InstancedStaticMeshComponent.AddInstance` (`self.InstancedStaticMesh`) (`KismetMathLibrary.MakeTransform` (`KismetMathLibrary.MakeVector` _returnvalue_4 _returnvalue_5) (struct) (`KismetMathLibrary.Conv_DoubleToVector` (`self.Scale`))) false))
        (bind _output_get_3 (set `local.InstanceIndex` _returnvalue_6))
        (`|ExecutionSequence`
          (:`then_0`
            (if (== _output_get_3 0)
              (set `self.First Transform` (`InstancedStaticMeshComponent.GetInstanceTransform` (`self.InstancedStaticMesh`) _output_get_3 false))))
          (:`then_1`
            (if (<= _returnvalue 0.0)
              (set `self.TileHeight` (* _returnvalue 5.0))
              (else
                (set `self.TileHeight` (`KismetMathLibrary.FClamp` _returnvalue 0.1))))
            (`InstancedStaticMeshComponent.UpdateInstanceTransform` (`self.InstancedStaticMesh`) (`local.InstanceIndex`) (`KismetMathLibrary.MakeTransform` (+ (.location (`InstancedStaticMeshComponent.GetInstanceTransform` (`self.InstancedStaticMesh`) (`local.InstanceIndex`) false)) (`KismetMathLibrary.MakeVector` 0.0 0.0 (+ (* (`self.TileHeight`) (`self.TileHeightStrength`)) (`self.TileHeightOffset`))))) false false false)
            (`InstancedStaticMeshComponent.SetCustomDataValue` (`self.InstancedStaticMesh`) (`local.InstanceIndex`) 0 (`self.TileHeight`) true)
            (if (== (`local.InstanceIndex`) (- (* (`self.Height`) (`self.Width`)) 1))
              (set `self.Final Transform` (`InstancedStaticMeshComponent.GetInstanceTransform` (`self.InstancedStaticMesh`) (`local.InstanceIndex`) false)))))
        (else
          (bind _returnvalue_7 (`AddComponent|NODE_AddChildActorComponent-2` :`RelativeTransform` (`KismetMathLibrary.MakeTransform` (`KismetMathLibrary.MakeVector` _returnvalue_4 _returnvalue_5) (struct) (`KismetMathLibrary.Conv_DoubleToVector` (`self.Scale`)))))
          (`ChildActorComponent.SetChildActorClass` _returnvalue_7 "/Game/HexGrid/BP_Tile.BP_Tile_C"))))
    (`/Engine/EditorBlueprintResources/StandardMacros.FlipFlop`
      (:`A`
        (set `self.RowOffset` (* (`self.Radius`) -1.0)))
      (:`B`
        (set `self.RowOffset` 0.0))))
  (`SceneComponent.K2_SetWorldTransform` (`self.StaticMesh`) (`KismetMathLibrary.MakeTransform` (`KismetMathLibrary.MakeVector` _returnvalue_x _returnvalue_y 25.0) (struct) (`KismetMathLibrary.MakeVector` (+ (`KismetMathLibrary.Conv_IntToDouble` (`self.Width`)) (`self.Radius`)) (+ (* (`KismetMathLibrary.Conv_IntToDouble` (`self.Height`)) 0.75) (`self.Radius`)) 1.0)) false false))